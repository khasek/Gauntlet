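; BP_Valkyrie is an actor that automatically melees nearby damageable actors while steadily damaging itself.
; A sphere overlap tracks actors implementing BPI_TakeDamage and updates the melee flags.
; A looping cooldown timer runs PerformMelee, which sends interface damage to the tracked actors, gated by those flags.
; A separate one-second looping timer applies engine damage to the actor itself.
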(event `self.ReceiveBeginPlay`
  (`KismetSystemLibrary.K2_SetTimer` null "PerformMelee" (`self.MeleeCooldown`) true)
  (`KismetSystemLibrary.K2_SetTimer` null "DamageOverTime" 1.0 true))

(event `self.Sphere.OnComponentBeginOverlap`
  (params (OverlappedComponent :type "PrimitiveComponent Object Reference") (OtherActor :type "Actor Object Reference") (OtherComp :type "PrimitiveComponent Object Reference") (OtherBodyIndex :type Integer) (bFromSweep :type Boolean) (SweepResult :type "HitResult Structure (by ref)"))
  (if (`KismetSystemLibrary.DoesImplementInterface` OtherActor "/Script/Gauntlet.BPI_TakeDamage")
    (`KismetArrayLibrary.Array_Add` (`self.OverlappedActors`) OtherActor)
    (set `self.CanMelee` true)))

(event `self.Sphere.OnComponentEndOverlap`
  (params (OverlappedComponent :type "PrimitiveComponent Object Reference") (OtherActor :type "Actor Object Reference") (OtherComp :type "PrimitiveComponent Object Reference") (OtherBodyIndex :type Integer))
  (bind _overlappedactors (`self.OverlappedActors`))
  (if (`KismetSystemLibrary.DoesImplementInterface` OtherActor "/Script/Gauntlet.BPI_TakeDamage")
    (set `self.StillOverlapped` false)
    (`KismetArrayLibrary.Array_RemoveItem` _overlappedactors OtherActor)
    (set `self.CanMelee` (`KismetArrayLibrary.Array_IsEmpty` _overlappedactors))))

(fn `DamageOverTime`
  (`GameplayStatics.ApplyDamage` self 1.0))

(fn `PerformMelee`
  (for _array_element (`self.OverlappedActors`)
    (if (`self.CanMelee`)
      (set `self.CanMelee` false)
      (set `self.StillOverlapped` true)
      (`KismetSystemLibrary.K2_SetTimer` null "ResetMelee" (`self.MeleeCooldown`))
      (message `BPI_TakeDamage.ApplyDamage` _array_element 1))
    (if (`self.StillOverlapped`)
      (set `self.CanMelee` true))))

(fn `UserConstructionScript`)