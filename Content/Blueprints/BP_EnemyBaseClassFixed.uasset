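; Base enemy Blueprint that sets an enemy's health from its level.
; On BeginPlay, SetStatsBasedOnLevel branches on EnemyLevel to assign Health, with any level other than the first two falling into the top tier.
; Move, Shoot, MeleeAttack and OnDeath are empty functions, and Tick and overlap events are unused, so no behavior or death handling is implemented here.
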(event `self.ReceiveBeginPlay`
  (`self.SetStatsBasedOnLevel`))

(fn `MeleeAttack`)

(fn `Move`)

(fn `OnDeath`)

(fn `SetStatsBasedOnLevel`
  (if (== (`self.EnemyLevel`) 1)
    (set `self.Health` 1)
    (elif (== (`self.EnemyLevel`) 2)
      (set `self.Health` 2)
      (else
        (set `self.Health` 3)))))

(fn `Shoot`)

(fn `UserConstructionScript`)