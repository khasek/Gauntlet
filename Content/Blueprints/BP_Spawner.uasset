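; Enemy spawner that releases one editor-selected enemy type (Grunt, Demon, Sorcerer, Lobber or Ghost) on a looping timer, using object pooling.
; BeginPlay pre-spawns the pool far above the level, hidden and without collision.
; SpawnFromPool teleports the first hidden enemy in front of the spawner, re-enables it and sets movement flags on the shared chase component for some types.
; ReturnToPool hides enemies, disables mesh collision and moves them away for reuse.
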(event `self.ReceiveBeginPlay`
  (bind _returnvalue (`KismetMathLibrary.MakeTransform` (0.0 0.0 100000.0)))
  (`KismetSystemLibrary.K2_SetTimer` null "SpawnFromPool" 5.0 true)
  (for _ (range (+ (`self.PoolSize`) 1))
    ;[0.4349 1 0] Dev sets enum in editor
    (switch `/Game/Blueprints/EEnemyType` (`self.Enemy`)
      (:`NewEnumerator0`
        ;[0.7016 0 1] Spawns relevent enemy
        (bind _returnvalue_2 (`|SpawnActorFromClass` (`self.GruntRef`) _returnvalue "Undefined" "OverrideRootScale" null null))
        ;[0.04079 0 1] Object pooling, pool size is determined in editor as well
        (bind _output_get (set `self.TempGrunt` _returnvalue_2))
        (`self.DisableAllMeshCollisions` _output_get)
        (`self.SetActorHiddenInGame` _output_get true)
        (`PrimitiveComponent.SetCollisionEnabled` (`/Game/Blueprints/BP_EnemyBaseClassFixed.BoxCollider` _output_get) "NoCollision")
        (`KismetArrayLibrary.Array_Add` (`self.EnemyPool`) _output_get))
      (:`NewEnumerator1`
        (bind _returnvalue_3 (`|SpawnActorFromClass` (`self.DemonRef`) _returnvalue "Undefined" "OverrideRootScale" null null 0 0 0 0 null))
        (set `/Game/Blueprints/BP_Enemy_Demon_Fixed.OwningSpawner` self _returnvalue_3)
        (bind _output_get_2 (set `self.TempDemon` _returnvalue_3))
        (`self.DisableAllMeshCollisions` _output_get_2)
        (`self.SetActorHiddenInGame` _output_get_2 true)
        (`PrimitiveComponent.SetCollisionEnabled` (`/Game/Blueprints/BP_EnemyBaseClassFixed.BoxCollider` _output_get_2) "NoCollision")
        (`KismetArrayLibrary.Array_Add` (`self.EnemyPool`) _output_get_2))
      (:`NewEnumerator2`
        (bind _returnvalue_4 (`|SpawnActorFromClass` (`self.Sorcerer`) _returnvalue "Undefined" "OverrideRootScale" null null))
        (bind _output_get_3 (set `self.TempSorcerer` _returnvalue_4))
        (`self.DisableAllMeshCollisions` _output_get_3)
        (`self.SetActorHiddenInGame` _output_get_3 true)
        (`PrimitiveComponent.SetCollisionEnabled` (`/Game/Blueprints/BP_EnemyBaseClassFixed.BoxCollider` _output_get_3) "NoCollision")
        (`KismetArrayLibrary.Array_Add` (`self.EnemyPool`) _output_get_3))
      (:`NewEnumerator3`
        (bind _returnvalue_5 (`|SpawnActorFromClass` (`self.Lobber`) _returnvalue "Undefined" "OverrideRootScale" null null))
        (bind _output_get_4 (set `self.TempLobber` _returnvalue_5))
        (`self.DisableAllMeshCollisions` _output_get_4)
        (`self.SetActorHiddenInGame` _output_get_4 true)
        (`PrimitiveComponent.SetCollisionEnabled` (`/Game/Blueprints/BP_EnemyBaseClassFixed.BoxCollider` _output_get_4) "NoCollision")
        (`KismetArrayLibrary.Array_Add` (`self.EnemyPool`) _output_get_4))
      (:`NewEnumerator4`
        (bind _returnvalue_6 (`|SpawnActorFromClass` (`self.GhostRef`) _returnvalue "Undefined" "OverrideRootScale" null null))
        (bind _output_get_5 (set `self.TempGhost` _returnvalue_6))
        (`self.DisableAllMeshCollisions` _output_get_5)
        (`self.SetActorHiddenInGame` _output_get_5 true)
        (`PrimitiveComponent.SetCollisionEnabled` (`/Game/Blueprints/BP_EnemyBaseClassFixed.BoxCollider` _output_get_5) "NoCollision")
        (`KismetArrayLibrary.Array_Add` (`self.EnemyPool`) _output_get_5)))))

(fn `DisableAllMeshCollisions`
  (params (TargetActor :type "Actor Object Reference"))
  (for _array_element (`self.K2_GetComponentsByClass` TargetActor "/Script/Engine.StaticMeshComponent")
    (`PrimitiveComponent.SetCollisionEnabled` _array_element "NoCollision")))

(fn `EnableAllMeshCollisions`
  (params (NewParam :type "Actor Object Reference"))
  (for _array_element (`self.K2_GetComponentsByClass` NewParam "/Script/Engine.StaticMeshComponent")
    (`PrimitiveComponent.SetCollisionEnabled` _array_element "QueryAndPhysics")))

(fn `ReturnToPool`
  (params (Actor :type "Actor Object Reference"))
  (`self.DisableAllMeshCollisions` Actor)
  (`self.SetActorHiddenInGame` Actor true)
  (`self.K2_SetActorLocation` Actor (0.0 0.0 100000.0) false false))

(fn `SpawnFromPool`
  (for _array_element (`self.EnemyPool`)
    (if (`Actor.bHidden` _array_element)
      (`self.K2_SetActorTransform` _array_element (`KismetMathLibrary.MakeTransform` (+ (* (`self.GetActorForwardVector`) (200.0 0.0 0.0)) (`self.K2_GetActorLocation`))) false true)
      (`self.EnableAllMeshCollisions` _array_element)
      (`PrimitiveComponent.SetCollisionEnabled` (`/Game/Blueprints/BP_EnemyBaseClassFixed.BoxCollider` _array_element) "QueryAndPhysics")
      (`self.SetActorHiddenInGame` _array_element false)
      ;[1 0.1369 0.3895] Enemies share same c++ movement class, this sets specific move patterns
      (switch `/Game/Blueprints/EEnemyType` (`self.Enemy`)
        (:`NewEnumerator0`
          (break))
        (:`NewEnumerator1`
          (bind _returnvalue (`self.GetComponentByClass` _array_element "/Script/Gauntlet.EightDirectionChaseComponent"))
          (set `EightDirectionChaseComponent.demonMovement` true _returnvalue)
          (break))
        (:`NewEnumerator2`
          (set `EightDirectionChaseComponent.sorcMovement` true _returnvalue)
          (break))
        (:`NewEnumerator3`
          (set `EightDirectionChaseComponent.lobberMovement` true _returnvalue)
          (break))
        (:`NewEnumerator4`
          (break))))))

(fn `UserConstructionScript`)