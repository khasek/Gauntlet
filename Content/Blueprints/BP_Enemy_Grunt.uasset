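; BP_Enemy_Grunt is an enemy Blueprint for a grunt type, built on a parent enemy class.
; It extends the parent's level-based stat setup by setting Damage in three tiers from EnemyLevel.
; BeginPlay, construction and death only call the parent.
; MeleeAttack, Move and Shoot are empty overrides with their parent calls left unconnected, so the parent behavior for those actions does not run.
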(event `self.ReceiveBeginPlay`
  (`parent.ReceiveBeginPlay`))

(event `self.ReceiveTick`
  (params (DeltaSeconds :type "Float (single-precision)")))

(fn `MeleeAttack`)

(fn `Move`)

(fn `OnDeath`
  (`parent.OnDeath`))

(fn `SetStatsBasedOnLevel`
  (`parent.SetStatsBasedOnLevel`)
  (if (== (`self.EnemyLevel`) 1)
    (set `self.Damage` 5)
    (elif (== (`self.EnemyLevel`) 2)
      (set `self.Damage` 8)
      (else
        (set `self.Damage` 10)))))

(fn `Shoot`)

(fn `UserConstructionScript`
  (`parent.UserConstructionScript`))