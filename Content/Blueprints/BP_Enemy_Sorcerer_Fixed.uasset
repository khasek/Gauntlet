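; Sorcerer enemy Blueprint, built on a parent enemy class, that sets its damage from its level across three tiers.
; Incoming damage reduces health and triggers death at zero or below.
; Death recomputes level stats and returns the enemy to its spawner's pool, bypassing the parent's death logic.
; Melee, movement and shooting overrides only call the parent implementations.
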(event `self.ApplyDamage`
  (params (dmgAmnt :type Integer))
  (bind _output_get (set `self.Health` (- (`self.Health`) dmgAmnt)))
  (if (<= _output_get 0)
    (`self.OnDeath`)))

(fn `MeleeAttack`
  (`parent.MeleeAttack`))

(fn `Move`
  (`parent.Move`))

(fn `OnDeath`
  (`self.SetStatsBasedOnLevel`)
  (`/Game/Blueprints/BP_Spawner.ReturnToPool` (`self.OwningSpawner`) self))

(fn `SetStatsBasedOnLevel`
  (`parent.SetStatsBasedOnLevel`)
  (if (== (`self.EnemyLevel`) 1)
    (set `self.Damage` 5)
    (elif (== (`self.EnemyLevel`) 2)
      (set `self.Damage` 8)
      (else
        (set `self.Damage` 10)))))

(fn `Shoot`
  (params (PlayerToShoot :type "Actor Object Reference"))
  (`parent.Shoot` null))

(fn `UserConstructionScript`
  (`parent.UserConstructionScript`))